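; Base enemy Blueprint for a node-based horror game, with empty hooks for actions, flashlight reactions and player teleports.
; Activate and Deactivate control a looping interval timer, and action checks roll 1–20 against Difficulty before calling TakeAction.
; Movement picks random connected nodes from the GameMode's node map and refuses blocked destinations, while JumpScare triggers game over.
; TimerCheck matches times against TimerNotifies through a DoOnce gate.
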(event `self.ReceiveBeginPlay`
  (bind _asgm_main (cast `/Game/GameManager/GM_Main` (`GameplayStatics.GetGameMode`)))
  (set `self.GameMode` _asgm_main)
  (bind _asbp_player_character (cast `/Game/Player/BP_PlayerCharacter` (`GameplayStatics.GetPlayerPawn` 0)))
  (set `self.Player` _asbp_player_character))

(event `Activate`
  (bind _returnvalue (`KismetSystemLibrary.K2_SetTimerDelegate` (`|CreateDelegate` :!event `CheckActionOpportunity`) (`self.Interval`) true))
  (set `self.IntervalTimer` _returnvalue))

(event `Deactivate`
  (`KismetSystemLibrary.K2_InvalidateTimerHandle` (`self.IntervalTimer`)))

(event `CheckActionOpportunity`
  (`/Engine/EditorBlueprintResources/StandardMacros.CompareInt` (`KismetMathLibrary.RandomIntegerInRange` 1 20) (`self.Difficulty`)
    (:`==`
      _)
    (:`<`
      _))
  (`self.TakeAction`))

(event `TakeAction`)

(event `FlashlightOn`)

(event `FlashlightOff`)

(event `GetFlashedTick`)

(event `MoveTo`
  (params (DestinationNode :type "/Game/BluePrints/MapNodes/E_Node Enum" :default "NewEnumerator0"))
  (if (not (`/Game/BluePrints/MapNodes/BP_Node.Blocked?` (`BlueprintMapLibrary.Map_Find` (`/Game/GameManager/GM_Main.AllNodes` (`self.GameMode`)) DestinationNode)))
    (set `self.CurrentNode` DestinationNode)))

(event `JumpScare`
  (`/Game/GameManager/GM_Main.GameOver` (`self.GameMode`) false))

(event `OnPlayerTeleport`
  (params (To :type "/Game/BluePrints/MapNodes/E_PlayerNode Enum" :default "NewEnumerator12")))

(fn `RandomDestinationFronNode`
  (params (FromNode :type "/Game/BluePrints/MapNodes/E_Node Enum" :default "NewEnumerator0"))
  (returns (ToNode :type "/Game/BluePrints/MapNodes/E_Node Enum"))
  (bind (_value _returnvalue) (`BlueprintMapLibrary.Map_Find` (`/Game/GameManager/GM_Main.AllNodes` (`self.GameMode`)) FromNode))
  (if _returnvalue
    (return (`KismetArrayLibrary.Array_Random` (`/Game/BluePrints/MapNodes/BP_Node.ConnectedNodes` _value)))))

(fn `Timer Check`
  (params (Time :type Integer))
  (returns (TimeIndex :type Integer))
  (bind (_arrayindex _arrayelement) (`/Engine/EditorBlueprintResources/StandardMacros.ReverseForEachLoop` (`self.TimerNotifies`))
    (:`LoopBody`
      (if (== _arrayelement Time)
        (`/Engine/EditorBlueprintResources/StandardMacros.DoOnce` false :!label _label
          (:`Completed`
            (return _arrayindex)))))
    (:`Completed`
      (goto _label :!via `Reset`))))

(fn `UserConstructionScript`)