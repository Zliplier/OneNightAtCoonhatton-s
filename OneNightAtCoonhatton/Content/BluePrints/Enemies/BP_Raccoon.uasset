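; Raccoon enemy that creeps toward a jumpscare as its Progress builds, and is pushed back by being flashed.
; Each action opportunity adds Difficulty to Progress, while GetFlashedTick removes one point at most every 0.1 seconds, floored at zero.
; CheckLevel picks the highest LevelThreshold reached through a reverse loop with DoOnce.
; Level changes reveal or hide four raccoon meshes, playing a sound per visible one, until the final level triggers JumpScare.
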(event `self.GetFlashedTick`
  (`parent.GetFlashedTick`)
  (`/Engine/EditorBlueprintResources/StandardMacros.DoOnce` false :!label _label
    (:`Completed`
      (`|ExecutionSequence`
        (:`then_0`
          (bind _result (`/Engine/EditorBlueprintResources/StandardMacros.DecrementInt` (`self.Progress`))
            (:`  `
              (if (<= _result 0)
                (set `self.Progress` 0)))))
        (:`then_1`
          (`self.CheckLevel`)
          (`KismetSystemLibrary.Delay` 0.1)
          (goto _label :!via `Reset`))))))

(event `self.CheckActionOpportunity`
  (`self.TakeAction`))

(event `self.TakeAction`
  (`parent.TakeAction`)
  (set `self.Progress` (+ (`self.Progress`) (`self.Difficulty`)))
  (`self.CheckLevel`))

(event `self.JumpScare`
  (`parent.JumpScare`))

(fn `CheckLevel`
  (bind (_arrayindex _arrayelement) (`/Engine/EditorBlueprintResources/StandardMacros.ReverseForEachLoop` (`self.LevelThreshold`))
    (:`LoopBody`
      (if (>= (`self.Progress`) _arrayelement)
        (`/Engine/EditorBlueprintResources/StandardMacros.DoOnce` false :!label _label
          (:`Completed`
            (if (!= _arrayindex (`self.Level`))
              (bind _output_get (set `self.Level` _arrayindex))
              (switch `int` _output_get
                (:`0`
                  (`self.UpdateRaccoonLevel` _output_get :!label _label_2))
                (:`1`
                  (goto _label_2))
                (:`2`
                  (goto _label_2))
                (:`3`
                  (goto _label_2))
                (:`4`
                  (goto _label_2))
                (:`5`
                  (`self.JumpScare`))))))))
    (:`Completed`
      (goto _label :!via `Reset`))))

(fn `UpdateRaccoonLevel`
  (params (Num :type Integer))
  (for (_array_element _array_index) (`|MakeArray` (`self.Mesh`) (`self.Rac2`) (`self.Rac3`) (`self.Rac4`))
    (if (<= _array_index (- Num 1))
      (`SceneComponent.SetVisibility` _array_element true false)
      (`GameplayStatics.PlaySoundAtLocation` "/Game/Assets/Sounds/Raccoon/junkkru_Cue.junkkru_Cue" (`self.K2_GetActorLocation`) (struct) 1.0 1.0 0.0 "/Game/Assets/Sounds/Attenuation/DoorAttenuation.DoorAttenuation" null null null)
      (else
        (`SceneComponent.SetVisibility` _array_element false false)))))

(fn `UserConstructionScript`
  (`parent.UserConstructionScript`)
  (`SceneComponent.SetVisibility` (`self.Rac3`) (`self.Visibility`) false)
  (`SceneComponent.SetVisibility` (`self.Rac2`) (`self.Visibility`) false)
  (`SceneComponent.SetVisibility` (`self.Mesh`) (`self.Visibility`) false)
  (`SceneComponent.SetVisibility` (`self.Rac4`) (`self.Visibility`) false))