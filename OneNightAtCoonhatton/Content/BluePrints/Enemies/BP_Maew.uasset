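; Maew is an animatronic-style enemy that roams between house nodes toward the player's left door, extending a parent enemy's movement and difficulty logic.
; Each action picks a connected node, mostly at random, with positional sounds on key moves, while being flashed sends it to HallwayM after a delay.
; At the door it hides its mesh and runs timers, retreating if the door is closed or jumpscaring a player there who lights the open doorway.
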(event `AtDoor`
  (`KismetSystemLibrary.K2_ClearAndInvalidateTimerHandle` (`self.IntervalTimer`))
  (bind _returnvalue (`KismetSystemLibrary.K2_SetTimerDelegate` (delegate `CheckDoorClosed`) 3.0 true))
  (set `self.IntervalTimer` _returnvalue)
  (bind _returnvalue_2 (`KismetSystemLibrary.K2_SetTimerDelegate` (`|CreateDelegate` :!event `JumpScare`) 15.0))
  (set `self.DoorJumpScareTimer` _returnvalue_2)
  (`SceneComponent.SetVisibility` (`self.Mesh`) false false))

(event `CheckDoorClosed`
  (`GameplayStatics.PlaySoundAtLocation` "/Game/Assets/Sounds/animatronicbreath_Cue.animatronicbreath_Cue" (`self.K2_GetActorLocation`) (struct) 1.0 1.0 15.0 "/Game/Assets/Sounds/Attenuation/DoorAttenuation.DoorAttenuation" null null null)
  (if (`/Game/BluePrints/Door/BP_Door_Left.DoorClosed?` (`/Game/GameManager/GM_Main.DoorLeft` (`self.GameMode`)))
    (`self.MoveTo` "NewEnumerator7")
    (`KismetSystemLibrary.K2_ClearAndInvalidateTimerHandle` (`self.IntervalTimer`))
    (`KismetSystemLibrary.K2_ClearAndInvalidateTimerHandle` (`self.DoorJumpScareTimer`))
    (bind _returnvalue (`KismetSystemLibrary.K2_SetTimerDelegate` (`|CreateDelegate` :!event `CheckActionOpportunity`) (`self.Interval`) true))
    (set `self.IntervalTimer` _returnvalue)
    (`SceneComponent.SetVisibility` (`self.Mesh`) true false)
    (`/Game/GameManager/GM_Main.PlaySoundAtNode` (`self.GameMode`) "/Game/Assets/Sounds/DoorFootsteps/DoorFootsteps_Cue.DoorFootsteps_Cue" "NewEnumerator3")))

(event `self.GetFlashedTick`
  (`parent.GetFlashedTick`)
  (if (`KismetSystemLibrary.K2_IsValidTimerHandle` (`self.IntervalTimer`))
    (`/Engine/EditorBlueprintResources/StandardMacros.DoOnce` false :!label _label
      (:`Completed`
        (`KismetSystemLibrary.Delay` 1.0)
        (`self.MoveTo` "NewEnumerator6")
        (goto _label :!via `Reset`)))))

(event `self.FlashlightOn`
  (`parent.FlashlightOn`)
  (switch `/Game/BluePrints/MapNodes/E_Node` (`self.CurrentNode`) :!label _label_2
    (:`NewEnumerator2`
      (if (and (`|EnumEquality` (`/Game/Player/BP_PlayerCharacter.PlayerNode` (`self.Player`)) "NewEnumerator14") (not (`/Game/BluePrints/Door/BP_Door_Left.DoorClosed?` (`/Game/GameManager/GM_Main.DoorLeft` (`self.GameMode`)))) (`/Game/BluePrints/Flashlight/BP_Flashlight.LightOn?` (`/Game/Player/BP_PlayerCharacter.FlashLight` (`self.Player`))))
        (`self.JumpScare`)))))

(event `self.OnPlayerTeleport`
  (params (To :type "/Game/BluePrints/MapNodes/E_PlayerNode Enum" :default "NewEnumerator12"))
  (`parent.OnPlayerTeleport` To)
  (switch `/Game/BluePrints/MapNodes/E_PlayerNode` To
    (:`NewEnumerator14`
      (goto _label_2))))

(event `self.MoveTo`
  (params (DestinationNode :type "/Game/BluePrints/MapNodes/E_Node Enum" :default "NewEnumerator0"))
  (bind _gamemode (`self.GameMode`))
  (bind _gamemode_2 (`self.GameMode`))
  (bind _currentnode (`self.CurrentNode`))
  (`|ExecutionSequence`
    (:`then_0`
      ;[1 1 1] Enter
      (switch `/Game/BluePrints/MapNodes/E_Node` DestinationNode
        (:`NewEnumerator2`
          (`self.AtDoor`)
          (`/Game/GameManager/GM_Main.PlaySoundAtNode` _gamemode_2 "/Game/Assets/Sounds/DoorFootsteps/DoorFootsteps_Cue.DoorFootsteps_Cue" "NewEnumerator2"))
        (:`NewEnumerator3`
          (`/Game/GameManager/GM_Main.PlaySoundAtNode` _gamemode_2 "/Game/Assets/Sounds/Footsteps/Footsteps_Cue.Footsteps_Cue" "NewEnumerator3"))
        (:`NewEnumerator10`
          (`/Game/GameManager/GM_Main.PlaySoundAtNode` _gamemode_2 "/Game/Assets/Sounds/Sound_Effects_-_Stairs_Cue.Sound_Effects_-_Stairs_Cue" "NewEnumerator10"))))
    (:`then_1`
      ;[1 1 1] Exit
      (switch `/Game/BluePrints/MapNodes/E_Node` _currentnode
        (:`NewEnumerator2`
          (`/Game/GameManager/GM_Main.PlaySoundAtNode` _gamemode "/Game/Assets/Sounds/DoorFootsteps/DoorFootsteps_Cue.DoorFootsteps_Cue" _currentnode))
        (:`NewEnumerator10`
          (`/Game/GameManager/GM_Main.PlaySoundAtNode` _gamemode "/Game/Assets/Sounds/Sound_Effects_-_Stairs_Cue.Sound_Effects_-_Stairs_Cue" _currentnode))))
    (:`then_2`
      (`parent.MoveTo` DestinationNode))))

(event `self.TakeAction`
  (`parent.TakeAction`)
  (switch `/Game/BluePrints/MapNodes/E_Node` (`self.CurrentNode`)
    (:`NewEnumerator3`
      (`self.MoveTo` (`self.RandomDestinationFronNode` (`self.CurrentNode`)) :!label _label_3))
    (:`NewEnumerator6`
      (`self.MoveTo` (select `int` (`KismetMathLibrary.RandomInteger` 1) :`0` "NewEnumerator7" :`1` "NewEnumerator9" :!type "/Game/BluePrints/MapNodes/E_Node Enum")))
    (:`NewEnumerator7`
      (`self.MoveTo` (select `int` (`KismetMathLibrary.RandomInteger` 2) :`0` "NewEnumerator10" :`1` "NewEnumerator6" :`2` "NewEnumerator3" :!type "/Game/BluePrints/MapNodes/E_Node Enum")))
    (:`NewEnumerator9`
      (goto _label_3))
    (:`NewEnumerator10`
      (goto _label_3))))

(fn `Timer Check`
  (params (Time :type Integer))
  (returns (TimeIndex :type Integer))
  (bind _difficulty (`self.Difficulty`))
  (bind _timeindex (`parent.Timer Check` Time))
  (`|ExecutionSequence`
    (:`then_0`
      (switch `int` _timeindex
        (:`0`
          (set `self.Difficulty` (+ _difficulty 3)))
        (:`1`
          (set `self.Difficulty` (+ _difficulty 3)))))
    (:`then_1`
      (return Time))))

(fn `UserConstructionScript`
  (`parent.UserConstructionScript`))