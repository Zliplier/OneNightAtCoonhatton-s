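; Left-hand door that is grabbed and swung with a motion controller through its GrabComponent.
; While held, each Tick sets the door's world yaw from a look-at between controller and door, clamped between MinDegrees and MaxDegrees.
; When released, its relative yaw steps down toward MinDegrees by a fixed amount per frame, independent of delta time.
; DoorClosed is true whenever world yaw is within a small tolerance of MaxDegrees.
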(event `self.ReceiveTick`
  (params (DeltaSeconds :type "Float (single-precision)"))
  (bind (_returnvalue_roll _returnvalue_pitch _returnvalue_yaw) (`KismetMathLibrary.BreakRotator` (`SceneComponent.K2_GetComponentRotation` (`self.Door`))))
  (bind (_relativerotation_roll _relativerotation_pitch _relativerotation_yaw) (`KismetMathLibrary.BreakRotator` (`SceneComponent.RelativeRotation` (`self.Door`))))
  (bind _motioncontrollerref (`/Game/Template/VRTemplate/Blueprints/GrabComponent.MotionControllerRef` (`self.GrabComponent`)))
  (bind (_returnvalue_roll_2 _returnvalue_pitch_2 _returnvalue_yaw_2) (`KismetMathLibrary.BreakRotator` (`KismetMathLibrary.FindLookAtRotation` (`SceneComponent.K2_GetComponentLocation` _motioncontrollerref) (`SceneComponent.K2_GetComponentLocation` (`self.Door`)))))
  (bind (_returnvalue_roll_3 _returnvalue_pitch_3 _returnvalue_yaw_3) (`KismetMathLibrary.BreakRotator` (`KismetMathLibrary.RLerp` (`KismetMathLibrary.MakeRotator` 0.0 0.0 (`self.MinDegrees`)) (`KismetMathLibrary.MakeRotator` 0.0 0.0 (`self.MaxDegrees`)) (/ (- (`KismetMathLibrary.ClampAngle` (+ _relativerotation_yaw -1.5) (`self.MinDegrees`) (`self.MaxDegrees`)) (`self.MinDegrees`)) (- (`self.MaxDegrees`) (`self.MinDegrees`))))))
  (`|ExecutionSequence`
    (:`then_0`
      (if (`/Game/Template/VRTemplate/Blueprints/GrabComponent.bIsHeld` (`self.GrabComponent`))
        (`/Engine/EditorBlueprintResources/StandardMacros.IsValid` _motioncontrollerref
          (:`Is Valid`
            (`SceneComponent.K2_SetWorldRotation` (`self.Door`) (`KismetMathLibrary.MakeRotator` 0.0 0.0 (`KismetMathLibrary.ClampAngle` (- _returnvalue_yaw_2 90.0) (`self.MinDegrees`) (`self.MaxDegrees`))) false false)))
        (else
          (`SceneComponent.K2_SetRelativeRotation` (`self.Door`) (`KismetMathLibrary.MakeRotator` 0.0 0.0 _returnvalue_yaw_3) false false))))
    (:`then_1`
      (if (`KismetMathLibrary.NearlyEqual_FloatFloat` _returnvalue_yaw (`self.MaxDegrees`) 5.0)
        (set `self.DoorClosed?` true)
        (else
          (set `self.DoorClosed?` false))))))

(fn `UserConstructionScript`)