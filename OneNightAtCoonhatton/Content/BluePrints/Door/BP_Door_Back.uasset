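; VR door that swings on its yaw axis when grabbed with a motion controller.
; While held, Tick aims the door from the controller's position, clamped to its angle limits.
; When not held, each tick offsets the current yaw slightly and lerps between the limits, rotating with a sweep.
; A DoorClosed flag plays the unlock sound whenever yaw enters or leaves a small tolerance around zero.
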(event `self.ReceiveTick`
  (params (DeltaSeconds :type "Float (single-precision)"))
  (bind (_returnvalue_roll _returnvalue_pitch _returnvalue_yaw) (`KismetMathLibrary.BreakRotator` (`SceneComponent.K2_GetComponentRotation` (`self.Door`))))
  (bind (_returnvalue_roll_2 _returnvalue_pitch_2 _returnvalue_yaw_2) (`KismetMathLibrary.BreakRotator` (`SceneComponent.K2_GetComponentRotation` (`self.Door`))))
  (bind _motioncontrollerref (`/Game/Template/VRTemplate/Blueprints/GrabComponent.MotionControllerRef` (`self.GrabComponent`)))
  (bind (_returnvalue_roll_3 _returnvalue_pitch_3 _returnvalue_yaw_3) (`KismetMathLibrary.BreakRotator` (`KismetMathLibrary.FindLookAtRotation` (`SceneComponent.K2_GetComponentLocation` _motioncontrollerref) (`SceneComponent.K2_GetComponentLocation` (`self.Door`)))))
  (bind (_returnvalue_roll_4 _returnvalue_pitch_4 _returnvalue_yaw_4) (`KismetMathLibrary.BreakRotator` (`KismetMathLibrary.RLerp` (`KismetMathLibrary.MakeRotator` 0.0 0.0 (`self.MinDegrees`)) (`KismetMathLibrary.MakeRotator` 0.0 0.0 (* (`self.MaxDegrees`) -1.0)) (/ (`KismetMathLibrary.ClampAngle` (+ (* _returnvalue_yaw -1.0) 1.5) (`self.MinDegrees`) (`self.MaxDegrees`)) (`self.MaxDegrees`)))))
  (`|ExecutionSequence`
    (:`then_0`
      (if (`/Game/Template/VRTemplate/Blueprints/GrabComponent.bIsHeld` (`self.GrabComponent`))
        (`/Engine/EditorBlueprintResources/StandardMacros.IsValid` _motioncontrollerref
          (:`Is Valid`
            (`SceneComponent.K2_SetWorldRotation` (`self.Door`) (`KismetMathLibrary.MakeRotator` 0.0 0.0 (`KismetMathLibrary.ClampAngle` (- _returnvalue_yaw_3 90.0) (* (`self.MaxDegrees`) -1.0) (`self.MinDegrees`))) false false)))
        (else
          (`SceneComponent.K2_SetWorldRotation` (`self.Door`) (`KismetMathLibrary.MakeRotator` 0.0 0.0 _returnvalue_yaw_4) true false))))
    (:`then_1`
      (if (`KismetMathLibrary.NearlyEqual_FloatFloat` _returnvalue_yaw_2 0.0 5.0)
        (if (not (`self.DoorClosed?`))
          (set `self.DoorClosed?` true)
          (`GameplayStatics.PlaySoundAtLocation` "/Game/Assets/Sounds/doorunlock_Cue.doorunlock_Cue" (`self.K2_GetActorLocation`) (struct) 1.0 1.0 0.0 "/Game/Assets/Sounds/Attenuation/DoorAttenuation.DoorAttenuation" null null null :!label _label))
        (elif (`self.DoorClosed?`)
          (set `self.DoorClosed?` false)
          (goto _label))))))

(fn `UserConstructionScript`)