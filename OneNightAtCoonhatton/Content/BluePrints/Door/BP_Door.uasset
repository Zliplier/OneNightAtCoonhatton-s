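; BP_Door is a VR door that swings to follow the motion controller holding it.
; While GrabComponent is held, Tick sets the door's world yaw from the look-at angle between controller and door, offset and clamped to a half-turn range.
; When released, the door snaps to zero world rotation if it is near that yaw, and otherwise stays where it was left.
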(event `self.ReceiveTick`
  (params (DeltaSeconds :type "Float (single-precision)"))
  (bind (_returnvalue_roll _returnvalue_pitch _returnvalue_yaw) (`KismetMathLibrary.BreakRotator` (`SceneComponent.K2_GetComponentRotation` (`self.Door`))))
  (bind _motioncontrollerref (`/Game/Template/VRTemplate/Blueprints/GrabComponent.MotionControllerRef` (`self.GrabComponent`)))
  (bind (_returnvalue_roll_2 _returnvalue_pitch_2 _returnvalue_yaw_2) (`KismetMathLibrary.BreakRotator` (`KismetMathLibrary.FindLookAtRotation` (`SceneComponent.K2_GetComponentLocation` _motioncontrollerref) (`SceneComponent.K2_GetComponentLocation` (`self.Door`)))))
  (if (`/Game/Template/VRTemplate/Blueprints/GrabComponent.bIsHeld` (`self.GrabComponent`))
    (`/Engine/EditorBlueprintResources/StandardMacros.IsValid` _motioncontrollerref
      (:`Is Valid`
        (`SceneComponent.K2_SetWorldRotation` (`self.Door`) (`KismetMathLibrary.MakeRotator` 0.0 0.0 (`KismetMathLibrary.ClampAngle` (- _returnvalue_yaw_2 90.0) -90.0 90.0)) false false)))
    (elif (`KismetMathLibrary.NearlyEqual_FloatFloat` _returnvalue_yaw 0.0 10.0)
      (`SceneComponent.K2_SetWorldRotation` (`self.Door`) (struct) false false))))

(fn `UserConstructionScript`)