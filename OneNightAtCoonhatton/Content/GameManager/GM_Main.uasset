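; GM_Main is the game manager for a timed night of surviving enemies.
; A looping timer advances the in-game clock and reports time to enemies; reaching hour six wins.
; Game over deactivates enemies, then opens the cutscene map on a win or the lobby on a loss.
; It relays flashlight, teleport and flash events to enemies, briefly blocks flashed nodes and plays sounds at node locations.
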(event `self.ReceiveBeginPlay`)

(event `StartNight`
  (bind _allenemies (`self.AllEnemies`))
  (bind (_value _returnvalue) (`BlueprintMapLibrary.Map_Find` _allenemies "NewEnumerator0"))
  (bind _returnvalue_2 (`KismetSystemLibrary.K2_SetTimerDelegate` (`|CreateDelegate` :!event `GameTick`) (`self.MinGameToIrl`) true))
  (set `self.NightTimer` _returnvalue_2)
  (if (and _returnvalue (`.ReturnValue` (`BlueprintMapLibrary.Map_Find` _allenemies "NewEnumerator1")) (`.ReturnValue` (`BlueprintMapLibrary.Map_Find` _allenemies "NewEnumerator2")))
    (`/Game/BluePrints/Enemies/BP_Enemy.Activate` _value)
    (`/Game/BluePrints/Enemies/BP_Enemy.Activate` (`BlueprintMapLibrary.Map_Find` _allenemies "NewEnumerator1"))
    (`/Game/BluePrints/Enemies/BP_Enemy.Activate` (`BlueprintMapLibrary.Map_Find` _allenemies "NewEnumerator2"))))

(event `GameOver`
  (params (`Win?` :type Boolean))
  (`/Engine/EditorBlueprintResources/StandardMacros.DoOnce` false
    (:`Completed`
      (`|ExecutionSequence`
        (:`then_0`
          (bind _values (`BlueprintMapLibrary.Map_Values` (`self.AllEnemies`)))
          (for _array_element _values
            (`/Game/BluePrints/Enemies/BP_Enemy.Deactivate` _array_element))
          (`KismetSystemLibrary.K2_ClearAndInvalidateTimerHandle` (`self.NightTimer`)))
        (:`then_1`
          (if `Win?`
            (`KismetSystemLibrary.Delay` 2.5)
            (`GameplayStatics.OpenLevelBySoftObjectPtr` "/Game/RaccoonzONLY/CutSceneMap.CutSceneMap")
            (else
              (`KismetSystemLibrary.Delay` 2.5)
              (`GameplayStatics.OpenLevelBySoftObjectPtr` "/Game/Level/Lobby.Lobby"))))))))

(event `GameTick`
  (`self.Minute Tick`)
  (`self.TimeNotify`))

(event `FlashlightOpen`
  (bind _values (`BlueprintMapLibrary.Map_Values` (`self.AllEnemies`)))
  (for _array_element _values
    (`/Game/BluePrints/Enemies/BP_Enemy.FlashlightOn` _array_element)))

(event `FlashlightClose`
  (bind _values (`BlueprintMapLibrary.Map_Values` (`self.AllEnemies`)))
  (for _array_element _values
    (`/Game/BluePrints/Enemies/BP_Enemy.FlashlightOff` _array_element)))

(event `OnTeleport`
  (params (To :type "/Game/BluePrints/MapNodes/E_PlayerNode Enum" :default "NewEnumerator12"))
  (bind _values (`BlueprintMapLibrary.Map_Values` (`self.AllEnemies`)))
  (for _array_element _values
    (`/Game/BluePrints/Enemies/BP_Enemy.OnPlayerTeleport` _array_element To)))

(event `Flash`
  (params (Node :type "/Game/BluePrints/MapNodes/E_Node Enum" :default "NewEnumerator0"))
  (bind (_value _returnvalue) (`BlueprintMapLibrary.Map_Find` (`self.AllNodes`) Node))
  (`|ExecutionSequence`
    (:`then_0`
      (bind _values (`BlueprintMapLibrary.Map_Values` (`self.AllEnemies`)))
      (for _array_element _values
        (if (`|EnumEquality` (`/Game/BluePrints/Enemies/BP_Enemy.CurrentNode` _array_element) Node)
          (`/Game/BluePrints/Enemies/BP_Enemy.GetFlashedTick` _array_element))))
    (:`then_1`
      (if _returnvalue
        (set `/Game/BluePrints/MapNodes/BP_Node.Blocked?` true _value)
        (`KismetSystemLibrary.RetriggerableDelay` 0.2)
        (set `/Game/BluePrints/MapNodes/BP_Node.Blocked?` false _value)))))

(event `PlaySoundAtNode`
  (params (Sound :type "SoundBase Object Reference") (Node :type "/Game/BluePrints/MapNodes/E_Node Enum" :default "NewEnumerator0"))
  (bind (_value _returnvalue) (`BlueprintMapLibrary.Map_Find` (`self.AllNodes`) Node))
  (if _returnvalue
    (`GameplayStatics.PlaySoundAtLocation` Sound (`self.K2_GetActorLocation` _value) (struct) 1.0 1.0 0.0 "/Game/Assets/Sounds/Attenuation/GlobalAttenuation.GlobalAttenuation" null null null)))

(fn `Minute Tick`
  (bind _result (`/Engine/EditorBlueprintResources/StandardMacros.IncrementInt` (`self.Minute`))
    (:`  `
      (if (>= _result 60)
        (set `self.Minute` 0)
        (bind _result_2 (`/Engine/EditorBlueprintResources/StandardMacros.IncrementInt` (`self.Hour`))
          (:`  `
            (if (>= _result_2 6)
              (`self.GameOver` true))))))))

(fn `TimeNotify`
  (bind _values (`BlueprintMapLibrary.Map_Values` (`self.AllEnemies`)))
  (for _array_element _values
    (`/Game/BluePrints/Enemies/BP_Enemy.Timer Check` _array_element (+ (`self.Minute`) (* (`self.Hour`) 60)))))

(fn `UserConstructionScript`)